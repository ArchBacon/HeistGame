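; BP_Drill is a heist-game drill that removes its referenced Vault when drilling completes.
; While active, it advances its progress every Tick.
; A handler bound to OnProgressCompleted at BeginPlay destroys the Vault, then the drill itself.
; The construction script refreshes the mesh materials and widget location.
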(event Custom|OnProgressCompleted_Event_0
  (Actor|DestroyActor (Variables|Default|GetVault))
  (Actor|DestroyActor))

(event EventBeginPlay
  (EventDispatchers|AssignOnProgressCompleted (delegate Custom|OnProgressCompleted_Event_0)))

(event EventTick
  (params (DeltaSeconds :type Float%20%28single-precision%29))
  (if (Class|Interactable|IsActive)
    (Class|Interactable|UpdateProgress DeltaSeconds)))

(fn ConstructionScript
  (Class|Interactable|UpdateMaterialsonMesh)
  (Class|Interactable|UpdateWidgetLocation))