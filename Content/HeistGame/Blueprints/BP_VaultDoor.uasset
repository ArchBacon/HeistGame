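; BP_VaultDoor is the vault door in the heist game, which accepts a thermal drill delivered in a duffle bag.
; Each Tick it scans its Box for overlapping duffle bags that are active and contain a ThermalDrill.
; A matching bag is destroyed, a BP_Drill spawns at the DrillLocation transform with a reference to the vault, and the diagonal-stripes placement sprite is hidden.
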(event EventTick
  (params (DeltaSeconds :type Float%20%28single-precision%29))
  (bind _drilllocation (Variables|Default|GetDrillLocation))
  (for _array_element (Collision|GetOverlappingActors (Variables|Default|GetBox) "/Game/HeistGame/Blueprints/BP_DuffleBag.BP_DuffleBag_C" :!class /Script/Engine.PrimitiveComponent)
    (bind _asbp_duffle_bag (Utilities|Casting|CastToBP_DuffleBag _array_element))
    (if (and (Class|Interactable|IsActive _asbp_duffle_bag) (Utilities|Enum|Equal(Enum) (Default|GetContents _asbp_duffle_bag) "ThermalDrill"))
      (Actor|DestroyActor _asbp_duffle_bag)
      (bind _returnvalue (Game|SpawnActorfromClass "/Game/HeistGame/Blueprints/BP_Drill.BP_Drill_C" (Math|Transform|MakeTransform (Transformation|GetWorldLocation _drilllocation) (Transformation|GetWorldRotation _drilllocation) (Transformation|GetWorldScale _drilllocation)) "Undefined" 0 0))
      (Variables|/Game/HeistGame/Blueprints/BP_Drill.BP_Drill_C|SetVault _returnvalue self)
      (Rendering|SetVisibility (Variables|Default|Getdiagonal-stripes_600x_Sprite) false false))))

(fn ConstructionScript)