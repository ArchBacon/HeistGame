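; BP_DuffleBag is a loot bag pickup in the heist game that the player collects by completing a progress interaction.
; On completion it reactivates and refreshes its materials, then checks player 0's BP_HeistCharacter, using the carried bag's visibility as the already-carrying test.
; If none is carried, it copies its contents to the character, shows the bag, destroys itself and prints the pickup.
; The construction script updates materials and widget location.
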(event Custom|OnProgressCompleted_Event_0
  (Class|Interactable|SetActive true)
  (Class|Interactable|UpdateMaterialsonMesh)
  (bind _asbp_heist_character (Utilities|Casting|CastToBP_HeistCharacter (Game|GetPlayerCharacter 0)))
  (if (not (Rendering|IsVisible (Variables|/Game/HeistGame/Characters/BP_HeistCharacter.BP_HeistCharacter_C|GetBag _asbp_heist_character)))
    (Variables|/Script/HeistGame.HeistCharacter|SetBagContents _asbp_heist_character (Class|DuffleBag|GetContents))
    (Rendering|SetVisibility (Variables|/Game/HeistGame/Characters/BP_HeistCharacter.BP_HeistCharacter_C|GetBag _asbp_heist_character) true false)
    (Actor|DestroyActor)
    (Development|PrintString (Utilities|String|Append "Picked up " (Utilities|String|EnumtoString (Class|DuffleBag|GetContents))))))

(event EventBeginPlay
  (EventDispatchers|AssignOnProgressCompleted (delegate Custom|OnProgressCompleted_Event_0)))

(fn ConstructionScript
  (Class|Interactable|UpdateMaterialsonMesh)
  (Class|Interactable|UpdateWidgetLocation))