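; CCTV security camera that projects a BP_CCTV_Zone actor where it looks and colors itself red while active, grey otherwise.
; On BeginPlay an active camera spawns the zone at a forward line-trace hit, randomizing its starting yaw if rotation is enabled.
; Tick sweeps the camera within its rotation radius, pausing at each end, and moves the zone to follow.
; Completing the progress interaction destroys the zone.
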(event Custom|OnMaterialsUpdated_Event_0
  (CallFunction|UpdateMaterialsonCamera))

(event Custom|OnProgressCompleted_Event_0
  (bind _cctvzone (Variables|Default|GetCCTVZone)
    (:then
      (Actor|DestroyActor _cctvzone))
    (:else)))

(event EventTick
  (params (DeltaSeconds :type Float%20%28single-precision%29))
  (if (and (Variables|Default|GetbShouldRotate) (Class|Interactable|IsActive))
    (|RotateCamera)
    (bind _location (CallFunction|FindZoneLocation))
    (Transformation|SetActorLocation (Variables|Default|GetCCTVZone) _location false false)
    (Transformation|SetActorRotation (Variables|Default|GetCCTVZone) (Math|Rotator|MakeRotator 0.0 0.0 (.yaw (Transformation|GetWorldRotation (Variables|Default|GetSM_Camera)))))))

(event EventBeginPlay
  (bind _sm_camera (Variables|Default|GetSM_Camera))
  (bind _rotationradius (Variables|Default|GetRotationRadius))
  (bind _returnvalue (Transformation|GetWorldRotation _sm_camera))
  (EventDispatchers|AssignOnMaterialsUpdated (delegate Custom|OnMaterialsUpdated_Event_0))
  (Class|Interactable|UpdateMaterialsonMesh)
  (if (Class|Interactable|IsActive)
    (EventDispatchers|AssignOnProgressCompleted (delegate Custom|OnProgressCompleted_Event_0))
    (bind _location (CallFunction|FindZoneLocation))
    (bind _returnvalue_2 (Game|SpawnActorfromClass "/Game/HeistGame/Blueprints/CCTV/BP_CCTV_Zone.BP_CCTV_Zone_C" (Math|Transform|MakeTransform _location (Math|Rotator|MakeRotator 0.0 0.0 (.yaw (Transformation|GetWorldRotation (Variables|Default|GetSM_Camera)))) "1,1,1") "Undefined" 0 0))
    (Variables|Default|SetCCTVZone _returnvalue_2)
    (if (Variables|Default|GetbShouldRotate)
      (bind _output_get (Variables|Default|SetRotatedRadius (Math|Random|RandomFloatinRange (* _rotationradius -1.0) _rotationradius)))
      (Transformation|SetWorldRotation _sm_camera (Math|Rotator|MakeRotator 0.0 (.pitch _returnvalue) (+ (.yaw _returnvalue) _output_get)) false false))))

(fn ConstructionScript
  (bind _sm_camera (Variables|Default|GetSM_Camera))
  (bind _returnvalue (Transformation|GetWorldRotation _sm_camera))
  (Class|Interactable|UpdateMaterialsonMesh)
  (Class|Interactable|UpdateWidgetLocation)
  (|FixCameraHeight)
  (CallFunction|UpdateMaterialsonCamera)
  (Transformation|SetWorldRotation _sm_camera (Math|Rotator|MakeRotator 0.0 (.pitch _returnvalue) (+ (.yaw _returnvalue) (Variables|Default|GetRotatedRadius))) false false))

(fn UpdateMaterialsonCamera
  (bind _sm_camera (Variables|Default|GetSM_Camera))
  (for (_ _array_index) (Rendering|Material|GetMaterials _sm_camera)
    (Rendering|Material|SetMaterial _sm_camera _array_index (select (Class|Interactable|IsActive) "/Game/HeistGame/Materials/M_Red.M_Red" "/Game/HeistGame/Materials/M_grey.M_grey"))))

(fn FindZoneLocation
  (bind _sm_camera (Variables|Default|GetSM_Camera))
  (bind _returnvalue (Transformation|GetWorldLocation _sm_camera))
  (bind (_outhit _returnvalue_2) (Collision|LineTraceByChannel (+ _returnvalue "0, 0,15.000000") (+ _returnvalue (* (Math|Vector|GetForwardVector _sm_camera) 2e+03)) "TraceTypeQuery4" false 0 "ForOneFrame"))
  (if _returnvalue_2
    (return (.Location (Collision|BreakHitResult _outhit)))))