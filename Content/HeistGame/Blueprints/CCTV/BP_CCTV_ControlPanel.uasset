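; BP_CCTV_ControlPanel is a control panel that completes the progress of every CCTV in the level when its own progress finishes.
; On BeginPlay it caches all BP_CCTV actors and binds to its OnProgressCompleted event, which then calls CompleteProgress on each valid camera.
; The construction script updates the mesh materials and the widget location.
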(event Custom|OnProgressCompleted_Event_0
  (for _array_element (Variables|Default|GetCCTVs)
    (Utilities|IsValid _array_element
      (:Is%20Valid
        (Class|Interactable|CompleteProgress _array_element)))))

(event EventBeginPlay
  (bind _outactors (Actor|GetAllActorsOfClass "/Game/HeistGame/Blueprints/CCTV/BP_CCTV.BP_CCTV_C"))
  (Variables|Default|SetCCTVs _outactors)
  (EventDispatchers|AssignOnProgressCompleted (delegate Custom|OnProgressCompleted_Event_0)))

(fn ConstructionScript
  (Class|Interactable|UpdateMaterialsonMesh)
  (Class|Interactable|UpdateWidgetLocation))